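; BP_Projectile is a projectile actor that explodes about one second after it starts ticking.
; Tick runs a one-second Delay into the Explode event, acting as a fuse timer.
; Explode spawns the P_Explosion emitter at the actor's location and sets it to replicate, applies radial damage within DamageRadius credited to the instigator controller, then destroys the actor.
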(event Custom|Explode
  (bind _returnvalue (Transformation|GetActorLocation))
  (bind _returnvalue_2 (Effects|SpawnEmitteratLocation "/Game/WeaponEffects/Explosion/P_Explosion.P_Explosion" _returnvalue))
  (Class|ActorComponent|SetIsReplicated _returnvalue_2 true)
  (Game|Damage|ApplyRadialDamage 1e+02 _returnvalue (Variables|Default|GetDamageRadius) 0 0 self (Game|GetInstigatorController) false "ECC_Visibility")
  (Actor|DestroyActor))

(event EventTick
  (params (DeltaSeconds :type Float%20%28single-precision%29))
  (Utilities|FlowControl|Delay 1.0)
  (CallFunction|Explode))

(fn ConstructionScript)