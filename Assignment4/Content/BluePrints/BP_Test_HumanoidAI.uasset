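; BP_Test_HumanoidAI is a test humanoid AI character whose BeginPlay, death event and Tick are all empty, so its graph logic never runs.
; Disconnected nodes would start behavior tree Test_BT_V2, set the player pawn as blackboard TargetActor and bind the death event.
; A second orphaned chain would release the blackboard's CoverSpotV2 if this character occupies it, then disable movement avoidance.
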(event Custom|On_Death_Event
  (params (actor :type TPS%20Character%20Object%20Reference)))

(event EventBeginPlay)

(event EventTick
  (params (DeltaSeconds :type Float%20%28single-precision%29)))

(fn ConstructionScript)